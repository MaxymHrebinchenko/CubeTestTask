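; Cube pawn for a mark-and-clean task, with Cleaner, Normal and Marked types shown by material.
; On hitting another cube pawn, Marked spreads to Normal and Cleaner resets Marked to Normal, notifying BP_GameModeTask through Mark or Clear.
; A shared IsInteracted flag stops both cubes resolving the same collision.
; The construction script applies the starting material and turns Marked placements into Normal.
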(event `self.ReceiveBeginPlay`
  (bind _asbp_game_mode_task (cast `/Game/Task/Blueprints/BP_GameModeTask` (`GameplayStatics.GetGameMode`)))
  (set `self.GameMode` _asbp_game_mode_task))

(event `self.Cube.OnComponentHit`
  (params (HitComponent :type "PrimitiveComponent Object Reference") (OtherActor :type "Actor Object Reference") (OtherComp :type "PrimitiveComponent Object Reference") (NormalImpulse :type "Vector Structure") (Hit :type "HitResult Structure (by ref)"))
  (bind _gamemode (`self.GameMode`))
  ;[1 1 1] Pawn types interaction logic
  (bind _asbp_cube_pawn (cast `/Game/Task/Blueprints/BP_CubePawn` OtherActor))
  (if (`/Game/Task/Blueprints/BP_CubePawn.IsInteracted` _asbp_cube_pawn)
    (`self.SetStates` _asbp_cube_pawn)
    (else
      (`self.SetStates` _asbp_cube_pawn true
        (:`FlowOut`
          (switch `/Game/Task/Enum/BP_CubeTypes` (`self.CubeType`)
            (:`NewEnumerator0`
              (bind (_cleaner _normal _marked) (`self.EnumToBool` (`/Game/Task/Blueprints/BP_CubePawn.CubeType` _asbp_cube_pawn)))
              ;;[1 1 1] Better way to organize???
              (if _marked
                (`/Game/Task/Blueprints/BP_Paint.Paint` _asbp_cube_pawn "NewEnumerator1")
                (`/Game/Task/Blueprints/BP_GameModeTask.Clear` _gamemode :!label _label)))
            (:`NewEnumerator1`
              (if _marked
                (`/Game/Task/Blueprints/BP_Paint.Paint` "NewEnumerator2")
                (`/Game/Task/Blueprints/BP_GameModeTask.Mark` _gamemode :!label _label_2)))
            (:`NewEnumerator2`
              (if _cleaner
                (`/Game/Task/Blueprints/BP_Paint.Paint` "NewEnumerator1")
                (goto _label)
                (elif _normal
                  (`/Game/Task/Blueprints/BP_Paint.Paint` _asbp_cube_pawn "NewEnumerator2")
                  (goto _label_2))))))))))

(event `/Game/Task/Blueprints/BP_Paint.Paint`
  (params (Type :type "/Game/Task/Enum/BP_CubeTypes Enum" :default "NewEnumerator0"))
  (bind _cube (`self.Cube`))
  ;[1 1 1] Painting logic
  (switch `/Game/Task/Enum/BP_CubeTypes` Type
    (:`NewEnumerator1`
      (`PrimitiveComponent.SetMaterial` _cube 0 "/Game/Task/Materials/M_Cube.M_Cube")
      (set `self.CubeType` Type))
    (:`NewEnumerator2`
      (`PrimitiveComponent.SetMaterial` _cube 0 "/Game/Task/Materials/M_Player.M_Player")
      (set `self.CubeType` Type))))

(fn `SetState`
  (params (State :type Boolean))
  (set `self.IsInteracted` State))

(fn `UserConstructionScript`
  (bind _cube (`self.Cube`))
  (switch `/Game/Task/Enum/BP_CubeTypes` (`self.CubeType`)
    (:`NewEnumerator0`
      (`PrimitiveComponent.SetMaterial` _cube 0 "/Game/Task/Materials/M_Cleaner.M_Cleaner"))
    (:`NewEnumerator1`
      (`PrimitiveComponent.SetMaterial` _cube 0 "/Game/Task/Materials/M_Cube.M_Cube"))
    (:`NewEnumerator2`
      (`PrimitiveComponent.SetMaterial` _cube 0 "/Game/Task/Materials/M_Cube.M_Cube")
      (set `self.CubeType` "NewEnumerator1"))))