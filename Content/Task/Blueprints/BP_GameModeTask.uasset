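; Game mode for a physics-sphere game that tracks marked cubes and ends the game once all are marked.
; On begin play it counts all cube pawns, tallies one cube type as cleaners and shows that number in a widget.
; Mark and Clear events adjust the marked count.
; Reaching the total removes the widget and input mapping, freezes the player sphere, hides its arrow and shows the win widget.
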(event `self.ReceiveBeginPlay`
  ;[1 1 1] Receiving amount of all cubes
  (bind _outactors (`GameplayStatics.GetAllActorsOfClass` "/Game/Task/Blueprints/BP_CubePawn.BP_CubePawn_C"))
  (for _array_element _outactors
    (if (`|EnumEquality` (`/Game/Task/Blueprints/BP_CubePawn.CubeType` _array_element) "NewEnumerator0")
      (`/Engine/EditorBlueprintResources/StandardMacros.IncrementInt` (`self.Cleaners`))))
  (set `self.AllCubes` (`KismetArrayLibrary.Array_Length` _outactors))
  (bind _returnvalue (`|CreateWidget` "/Game/Task/Widgets/BP_Cleaners.BP_Cleaners_C"))
  (bind _output_get (set `self.CleanersWidget` _returnvalue))
  (`/Game/Task/Widgets/BP_Cleaners.UpdateCleaners` _output_get (`self.Cleaners`))
  (`UserWidget.AddToViewport` _output_get 0))

(event `Mark`
  ;[1 1 1] Mark/Clear events to keep track of marked cubes
  (`/Engine/EditorBlueprintResources/StandardMacros.IncrementInt` (`self.Marked`)
    (:`  `
      (if (== (`self.Marked`) (`self.AllCubes`))
        (`self.GameEnd`)))))

(event `Clear`
  ;[1 1 1] Mark/Clear events to keep track of marked cubes
  (`/Engine/EditorBlueprintResources/StandardMacros.DecrementInt` (`self.Marked`)))

(event `GameEnd`
  ;[1 1 1] Game end logic
  (`Widget.RemoveFromParent` (`self.CleanersWidget`))
  (`EnhancedInputSubsystemInterface.RemoveMappingContext` (pcsubsystem `EnhancedInputLocalPlayerSubsystem` (`GameplayStatics.GetPlayerController` 0)) "/Game/Task/Input/IMC_Default.IMC_Default" (struct))
  (bind _asbp_sphere (cast `/Game/Task/Blueprints/BP_Sphere` (`GameplayStatics.GetPlayerPawn` 0)))
  (bind _sphere (`/Game/Task/Blueprints/BP_Sphere.Sphere` _asbp_sphere))
  (`PrimitiveComponent.SetPhysicsLinearVelocity` _sphere (0.0 0.0 0.0) false "None")
  (`PrimitiveComponent.SetSimulatePhysics` _sphere false)
  (`SceneComponent.SetVisibility` (`/Game/Task/Blueprints/BP_Sphere.Arrow` _asbp_sphere) false false)
  (bind _returnvalue (`|CreateWidget` "/Game/Task/Widgets/BP_WinWidget.BP_WinWidget_C"))
  (`UserWidget.AddToViewport` _returnvalue 0))

(fn `UserConstructionScript`)