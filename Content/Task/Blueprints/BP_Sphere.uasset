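; BP_Sphere is a moving ball that marks the cubes it hits and shows its horizontal motion with an arrow.
; Each tick the arrow yaws toward the sphere's planar velocity and stretches with its speed.
; Hits clear the jumping flag and repaint any BP_CubePawn not already of the marked type.
; Each repaint calls Mark on BP_GameModeTask, first decrementing its Cleaners count and widget if the cube was a cleaner.
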(event `self.ReceiveTick`
  (params (DeltaSeconds :type "Float (single-precision)"))
  (bind (_returnvalue_x _returnvalue_y) (`KismetMathLibrary.BreakVector` (`SceneComponent.GetComponentVelocity` (`self.Sphere`))))
  (bind (_returnvalue_x_2 _returnvalue_y_2) (`KismetMathLibrary.BreakVector` (`SceneComponent.GetComponentVelocity` (`self.Sphere`))))
  (bind (_returnvalue_x_3 _returnvalue_y_3) (`KismetMathLibrary.BreakVector` (`KismetMathLibrary.Normal` (`KismetMathLibrary.MakeVector` _returnvalue_x_2 _returnvalue_y_2))))
  ;[1 1 1] Arrow logic
  (`SceneComponent.SetRelativeScale3D` (`self.Arrow`) (`KismetMathLibrary.MakeVector` (/ (`KismetMathLibrary.VSize` (`KismetMathLibrary.MakeVector` _returnvalue_x _returnvalue_y)) 300.0) 2.0 2.0))
  (`SceneComponent.K2_SetRelativeRotation` (`self.Arrow`) (`KismetMathLibrary.MakeRotator` 0.0 0.0 (`KismetMathLibrary.GetYawPitchFromVector` (`KismetMathLibrary.MakeVector` _returnvalue_x_3 _returnvalue_y_3))) false false))

(event `self.Sphere.OnComponentHit`
  (params (HitComponent :type "PrimitiveComponent Object Reference") (OtherActor :type "Actor Object Reference") (OtherComp :type "PrimitiveComponent Object Reference") (NormalImpulse :type "Vector Structure") (Hit :type "HitResult Structure (by ref)"))
  (bind _gamemode (`self.GameMode`))
  ;[1 1 1] Mark logic
  (`|ExecutionSequence`
    (:`then_0`
      (set `self.IsJumping` false))
    (:`then_1`
      (bind _asbp_cube_pawn (cast `/Game/Task/Blueprints/BP_CubePawn` OtherActor))
      (bind _cubetype (`/Game/Task/Blueprints/BP_CubePawn.CubeType` _asbp_cube_pawn))
      (if (`|EnumInequality` _cubetype "NewEnumerator2")
        (if (`|EnumEquality` _cubetype "NewEnumerator0")
          (bind _result (`/Engine/EditorBlueprintResources/StandardMacros.DecrementInt` (`/Game/Task/Blueprints/BP_GameModeTask.Cleaners` _gamemode))
            (:`  `
              (`/Game/Task/Widgets/BP_Cleaners.UpdateCleaners` (`/Game/Task/Blueprints/BP_GameModeTask.CleanersWidget` _gamemode) _result))))
        (`/Game/Task/Blueprints/BP_Paint.Paint` _asbp_cube_pawn "NewEnumerator2")
        (`/Game/Task/Blueprints/BP_GameModeTask.Mark` (`self.GameMode`))))))

(event `self.ReceiveBeginPlay`
  ;[1 1 1] Get gamemode
  (bind _asbp_game_mode_task (cast `/Game/Task/Blueprints/BP_GameModeTask` (`GameplayStatics.GetGameMode`)))
  (set `self.GameMode` _asbp_game_mode_task))

(fn `UserConstructionScript`)